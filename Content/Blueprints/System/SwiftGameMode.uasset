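; SwiftGameMode is a game mode that ends the game once every Target actor in the level is destroyed.
; On BeginPlay it counts Target actors into MaxTargets, and the CheckTargets event compares DestroyedTargets, which is not incremented here, against that total.
; When reached, EndGame creates the GameEndMenu widget if needed, adds it to the viewport and switches to UI-only input focused on its Retry button.
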(event Custom|CheckTargets
  (if (>= (Variables|Default|GetDestroyedTargets) (Variables|Default|GetMaxTargets))
    (bind _asswift_game_mode (Utilities|Casting|CastToSwiftGameMode (Game|GetGameMode)))
    (CallFunction|EndGame _asswift_game_mode)))

(event EventBeginPlay
  (bind _outactors (Actor|GetAllActorsOfClass "/Game/Blueprints/Characters/Target.Target_C"))
  (Variables|Default|SetMaxTargets (+ (Utilities|Array|LastIndex _outactors) 1)))

(event EventTick
  (params (DeltaSeconds :type Float%20%28single-precision%29)))

(fn ConstructionScript)

(fn EndGame
  (Utilities|IsValid 0
    (:Is%20Valid
      _)
    (:Is%20Not%20Valid
      (bind _returnvalue (UserInterface|CreateWidget "/Game/Blueprints/System/UI/GameEndMenu.GameEndMenu_C"))
      (Variables|Default|SetGameEndMenuReference _returnvalue)))
  (Input|SetInputModeUIOnly (Game|GetPlayerController 0) (Variables|/Game/Blueprints/System/UI/GameEndMenu.GameEndMenu_C|GetRetryButton (Variables|Default|GetGameEndMenuReference)) "DoNotLock")
  (UserInterface|Viewport|AddtoViewport (Variables|Default|GetGameEndMenuReference) 0))