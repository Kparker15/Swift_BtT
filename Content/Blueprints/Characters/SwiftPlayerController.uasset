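; Player controller that turns touch, swipe and button input into jump and directional actions on the possessed BaseCharacter.
; A left-half touch jumps, while a right-half or extra touch opens a Tick gate that fires one directional action past a distance threshold.
; The second touch's screen-side check compares against zero, so it jumps whenever no jump is active.
; Pause input toggles game pause and a cached PauseMenu widget, switching input mode.
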(event Custom|StartSwipe
  (bind _startloc (Variables|Default|GetStartLoc))
  (bind (_x _y) (Math|Vector2D|BreakVector2D _startloc))
  (Utilities|FlowControl|Gate true) ; enters at Open
)

(event Custom|EndSwipe
  (bind _startloc (Variables|Default|GetStartLoc))
  (bind (_x _y) (Math|Vector2D|BreakVector2D _startloc))
  (Utilities|FlowControl|Gate true) ; enters at Close
)

(event EventTick
  (params (DeltaSeconds :type Float%20%28single-precision%29))
  (bind _startloc (Variables|Default|GetStartLoc))
  (bind (_x _y) (Math|Vector2D|BreakVector2D _startloc))
  (Utilities|FlowControl|Gate true
    (:Exit
      ;[1 1 1] Which touch event is initiating a swipe?
      (switch int (Variables|Default|GetSwipeFingerIndex)
        (:Default
          (CallFunction|EndSwipe :!label _label))
        (:0
          (goto _label))
        (:1
          ;[1 1 1] Check direction of a touch swipe (Compare starting location with current location)
          (Variables|Default|SetCurrentLoc (|Touch1_2))
          (if (and (< (.Y (Math|Vector2D|BreakVector2D (Variables|Default|GetCurrentLoc))) _y) (>= (Math|Float|Absolute(Float) (- (.Y (Math|Vector2D|BreakVector2D (Variables|Default|GetCurrentLoc))) _y)) (Variables|Default|GetThreshold))) :!label _label_2
            ;[1 1 1] Call event based on direction of swipe
            (bind _asbase_character (Utilities|Casting|CastToBaseCharacter (Pawn|GetControlledPawn)))
            (Default|UpAction _asbase_character)
            (CallFunction|EndSwipe :!label _label_3)
            (elif (and (> (.Y (Math|Vector2D|BreakVector2D (Variables|Default|GetCurrentLoc))) _y) (>= (Math|Float|Absolute(Float) (- (.Y (Math|Vector2D|BreakVector2D (Variables|Default|GetCurrentLoc))) _y)) (Variables|Default|GetThreshold)))
              (bind _asbase_character_2 (Utilities|Casting|CastToBaseCharacter (Pawn|GetControlledPawn)))
              (Default|DownAction _asbase_character_2)
              (goto _label_3)
              (elif (and (>= (Math|Float|Absolute(Float) (- (.X (Math|Vector2D|BreakVector2D (Variables|Default|GetCurrentLoc))) _x)) (Variables|Default|GetThreshold)) (> (.X (Math|Vector2D|BreakVector2D (Variables|Default|GetCurrentLoc))) _x))
                (bind _asbase_character_3 (Utilities|Casting|CastToBaseCharacter (Pawn|GetControlledPawn)))
                (Default|RightAction _asbase_character_3)
                (goto _label_3)
                (elif (and (>= (Math|Float|Absolute(Float) (- (.X (Math|Vector2D|BreakVector2D (Variables|Default|GetCurrentLoc))) _x)) (Variables|Default|GetThreshold)) (< (.X (Math|Vector2D|BreakVector2D (Variables|Default|GetCurrentLoc))) _x))
                  (bind _asbase_character_4 (Utilities|Casting|CastToBaseCharacter (Pawn|GetControlledPawn)))
                  (Default|LeftAction _asbase_character_4)
                  (goto _label_3))))))
        (:2
          (Variables|Default|SetCurrentLoc (|Touch2_2))
          (goto _label_2))))))

(event EventBeginPlay
  (Variables|Default|SetbShowMouseCursor false))

(event Input|ActionEvents|InputActionDownAction
  (params (Key :type Key%20Structure))
  (:Pressed
    (bind _asbase_character (Utilities|Casting|CastToBaseCharacter (Pawn|GetControlledPawn)))
    (Default|DownAction _asbase_character)))

(event Input|ActionEvents|InputActionLeftAction
  (params (Key :type Key%20Structure))
  (:Pressed
    (bind _asbase_character (Utilities|Casting|CastToBaseCharacter (Pawn|GetControlledPawn)))
    (Default|LeftAction _asbase_character)))

(event Input|ActionEvents|InputActionSwipeInput1
  (params (Key :type Key%20Structure))
  (bind _returnvalue (Game|GetPlayerController 0))
  (bind (_locationx _locationy) (Class|PlayerController|GetInputTouchState _returnvalue "Touch1"))
  (bind _returnvalue_2 (Math|Vector2D|MakeVector2D _locationx _locationy))
  (:Pressed
    ;[1 1 1] Is the Player initiating a jump or a swipe? has a jump already been initiated?
    (Variables|Default|SetSwipeFingerIndex 1)
    (if (> _locationx (Math|Conversions|ToFloat(Integer) (/ (.SizeX (HUD|GetViewportSize)) 2))) ; Which half of the screen has been touched?
      ;[1 1 1] A swipe has begun, call swipe event
      (Variables|Default|SetCurrentLoc _returnvalue_2 :!label _label)
      (bind _output_get (Variables|Default|SetStartLoc _returnvalue_2))
      (Variables|Default|SetPriorLoc _output_get)
      (CallFunction|StartSwipe)
      (elif (== (Variables|Default|GetJumpFingerIndex) 0) ; has a jump already been initiated?
        ;[1 1 1] A jump has been initiated, prevent another swipe event from starting a jump by setting jump index
        (bind _asbase_character (Utilities|Casting|CastToBaseCharacter (Pawn|GetControlledPawn)))
        (Default|StartJump _asbase_character)
        (Variables|Default|SetJumpFingerIndex 1)
        (else
          (goto _label)))))
  (:Released
    ;[1 1 1] End Swipe and if jump had been initiated by this touch event then end the jump
    (CallFunction|EndSwipe)
    (if (== (Variables|Default|GetJumpFingerIndex) 1)
      (bind _asbase_character_2 (Utilities|Casting|CastToBaseCharacter (Pawn|GetControlledPawn)))
      (Default|EndJump _asbase_character_2)
      (Variables|Default|SetJumpFingerIndex 0))))

(event Input|ActionEvents|InputActionSwipeInput2
  (params (Key :type Key%20Structure))
  (bind _returnvalue (Game|GetPlayerController 0))
  (bind (_locationx _locationy) (Class|PlayerController|GetInputTouchState _returnvalue "Touch2"))
  (bind _returnvalue_2 (Math|Vector2D|MakeVector2D _locationx _locationy))
  (:Pressed
    ;[1 1 1] Same logic as SwipeInput 1
    (Variables|Default|SetSwipeFingerIndex 2)
    (if (> 0.0 (Math|Conversions|ToFloat(Integer) (/ (.SizeX (HUD|GetViewportSize)) 2)))
      (Variables|Default|SetCurrentLoc _returnvalue_2 :!label _label)
      (bind _output_get (Variables|Default|SetStartLoc _returnvalue_2))
      (Variables|Default|SetPriorLoc _output_get)
      (CallFunction|StartSwipe)
      (elif (== (Variables|Default|GetJumpFingerIndex) 0)
        (bind _asbase_character (Utilities|Casting|CastToBaseCharacter (Pawn|GetControlledPawn)))
        (Default|StartJump _asbase_character)
        (Variables|Default|SetJumpFingerIndex 2)
        (else
          (goto _label)))))
  (:Released
    (CallFunction|EndSwipe)
    (if (== (Variables|Default|GetJumpFingerIndex) 2)
      (bind _asbase_character_2 (Utilities|Casting|CastToBaseCharacter (Pawn|GetControlledPawn)))
      (Default|EndJump _asbase_character_2)
      (Variables|Default|SetJumpFingerIndex 0))))

(event Input|ActionEvents|InputActionRightAction
  (params (Key :type Key%20Structure))
  (:Pressed
    (bind _asbase_character (Utilities|Casting|CastToBaseCharacter (Pawn|GetControlledPawn)))
    (Default|RightAction _asbase_character)))

(event Input|ActionEvents|InputActionUpAction
  (params (Key :type Key%20Structure))
  (:Pressed
    (bind _asbase_character (Utilities|Casting|CastToBaseCharacter (Pawn|GetControlledPawn)))
    (Default|UpAction _asbase_character)))

(event Input|ActionEvents|InputActionJump
  (params (Key :type Key%20Structure))
  (bind _returnvalue (Pawn|GetControlledPawn))
  (:Pressed
    (bind _asbase_character (Utilities|Casting|CastToBaseCharacter _returnvalue))
    (Default|StartJump _asbase_character))
  (:Released
    (bind _asbase_character_2 (Utilities|Casting|CastToBaseCharacter _returnvalue))
    (Default|EndJump _asbase_character_2)))

(event Input|ActionEvents|InputActionPause
  (params (Key :type Key%20Structure))
  (bind _pausemenureference (Variables|Default|GetpauseMenuReference))
  (:Pressed
    (if (not (Game|IsGamePaused))
      (Utilities|IsValid (Variables|Default|GetpauseMenuReference)
        (:Is%20Valid
          _)
        (:Is%20Not%20Valid
          (bind _returnvalue (UserInterface|CreateWidget "/Game/Blueprints/System/UI/PauseMenu.PauseMenu_C"))
          (Variables|Default|SetPauseMenuReference _returnvalue)))
      (Input|SetInputModeGameandUI (Game|GetPlayerController 0) (Variables|/Game/Blueprints/System/UI/PauseMenu.PauseMenu_C|GetResumeButton _pausemenureference) "DoNotLock" true)
      (UserInterface|Viewport|AddtoViewport _pausemenureference 0)
      (Game|SetGamePaused true)
      (else
        (Widget|RemovefromParent (Variables|Default|GetPauseMenuReference))
        (Game|SetGamePaused false)
        (Input|SetInputModeGameOnly (Game|GetPlayerController 0))))))

(fn ConstructionScript)