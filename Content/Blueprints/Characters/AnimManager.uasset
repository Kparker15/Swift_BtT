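; AnimManager is a component that drives Paper2D flipbook animation for its owning BaseCharacter.
; Each tick it maps the character's AnimState (movement, landing, wall and attack states) to a flipbook and looping flag.
; Airborne and wall-slide states use AirAnimCheck to choose rise, peak or fall from Z velocity, holding fall once it is showing until upward movement.
; SetAnimation changes and restarts the sprite only when the flipbook differs.
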(event EventBeginPlay
  ;[1 1 1] Get reference to owning character
  (bind _asbase_character (Utilities|Casting|CastToBaseCharacter (Components|GetOwner)))
  (Variables|Default|SetCharacter _asbase_character))

(event EventTick
  (params (DeltaSeconds :type Float%20%28single-precision%29))
  ;[1 1 1] Sets animation based on character's current animation state
  (switch Utilities|FlowControl|Switch|SwitchonAnimStates (Variables|/Game/Blueprints/Characters/BaseCharacter.BaseCharacter_C|GetAnimState (Variables|Default|GetCharacter))
    (:NewEnumerator15
      (CallFunction|SetAnimation (Variables|Default|GetIdle) true true))
    (:NewEnumerator0
      (CallFunction|SetAnimation (Variables|Default|GetRun) true true))
    (:NewEnumerator1
      (bind (_returnanim _islooping) (CallFunction|AirAnimCheck (Variables|Default|GetJumpRise) (Variables|Default|GetJumpPeak) (Variables|Default|GetJumpFall)))
      (CallFunction|SetAnimation _returnanim _islooping true))
    (:NewEnumerator11
      (CallFunction|SetAnimation (Variables|Default|GetLand) false true))
    (:NewEnumerator3
      (CallFunction|SetAnimation (Variables|Default|GetUpAttack) false true))
    (:NewEnumerator4
      (CallFunction|SetAnimation (Variables|Default|GetRightAttack) false true))
    (:NewEnumerator8
      (CallFunction|SetAnimation (Variables|Default|GetLeftAttack) false true))
    (:NewEnumerator10
      (CallFunction|SetAnimation (Variables|Default|GetDownAttack) false true))
    (:NewEnumerator18
      (bind (_returnanim_2 _islooping_2) (CallFunction|AirAnimCheck (Variables|Default|GetWallRise) (Variables|Default|GetWallPeak) (Variables|Default|GetWallFall)))
      (CallFunction|SetAnimation _returnanim_2 _islooping_2 true))
    (:NewEnumerator19
      (CallFunction|SetAnimation (Variables|Default|GetWallStop) false true))
    (:NewEnumerator21
      (CallFunction|SetAnimation (Variables|Default|GetAirDownAttack) false true))))

(fn SetAnimation
  (params (Flipbook :type Paper%20Flipbook%20Object%20Reference) (IsLooping :type Boolean) (PlayFromStart :type Boolean))
  ;[1 1 1] Sets character flipbook, whether it is looping, and plays it from start (image index 0)
  (if (!= Flipbook (Class|PaperFlipbookComponent|GetFlipbook (Variables|/Script/Paper2D.PaperCharacter|GetSprite (Variables|Default|GetCharacter))))
    (Sprite|SetFlipbook (Variables|/Script/Paper2D.PaperCharacter|GetSprite (Variables|Default|GetCharacter)) Flipbook)
    (Components|Timeline|SetLooping (Variables|/Script/Paper2D.PaperCharacter|GetSprite (Variables|Default|GetCharacter)) IsLooping)
    (if PlayFromStart
      (Components|Timeline|PlayfromStart (Variables|/Script/Paper2D.PaperCharacter|GetSprite (Variables|Default|GetCharacter))))))

(fn AirAnimCheck
  (params (Rise :type Paper%20Flipbook%20Object%20Reference) (Peak :type Paper%20Flipbook%20Object%20Reference) (Fall :type Paper%20Flipbook%20Object%20Reference))
  (bind _character (Variables|Default|GetCharacter))
  (bind _charactermovement (Variables|/Script/Engine.Character|GetCharacterMovement _character))
  (bind _velocity (Variables|/Script/Engine.MovementComponent|GetVelocity _charactermovement))
  (bind _z (Math|Vector|BreakVector _velocity))
  ;[1 1 1] Sets animation based on player z velocity
  (if (> _z 0.0)
    (return Rise true)
    (elif (and (!= Fall (Class|PaperFlipbookComponent|GetFlipbook (Variables|/Script/Paper2D.PaperCharacter|GetSprite (Variables|Default|GetCharacter)))) (> _z -2e+02))
      (return Peak false)
      (else
        (return Fall true)))))