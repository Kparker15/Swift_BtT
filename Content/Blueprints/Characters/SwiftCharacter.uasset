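; SwiftCharacter is the auto-running 2D sprite player character, with jump, slash and crouching slide attack, plus HUD creation and game-over on death.
; Tick moves it right unless wall-blocked, uses traces to cut jumps and hold slides under ceilings, and sets AnimState.
; AnimState selects an AbilityID, whose sprite-frame window gates box-trace hit checks that damage BaseCharacters.
; Up and left actions only print, and Bounce is empty.
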(event OnFinishedPlaying(Sprite)
  ;[1 1 1] Detect animation ending. Compare current animation with AnimManager variables
  (switch Utilities|FlowControl|Switch|SwitchonAnimStates (Variables|Default|GetAnimState)
    (:NewEnumerator4
      (Variables|Default|SetIsUsingAbility false))
    (:NewEnumerator10
      (Variables|Default|SetIsUsingAbility false)
      (Character|UnCrouch)
      (Transformation|AddLocalOffset (Variables|Default|GetSprite) (* (Variables|Default|GetCrouchDisplacement) -1.0) false false))))

(event Custom|StartAttack
  (Utilities|FlowControl|Gate true) ; enters at Open
)

(event Custom|EndAttack
  (Utilities|FlowControl|Gate true) ; enters at Close
)

(event EventTick
  (params (DeltaSeconds :type Float%20%28single-precision%29))
  (bind _sprite (Variables|Default|GetSprite))
  (if (not (Variables|Default|GetIsDead))
    (Utilities|FlowControl|Sequence
      (:then_0
        ;[1 1 1] Check if it is okay for player to move
        (bind _istouchingwall (CallFunction|CheckforWall))
        (if (not _istouchingwall)
          (Pawn|Input|AddMovementInput "1.000000, 0, 0" 1.0 false)
          (if (and (AI|Components|NavMovement|IsCrouching (Variables|Character|GetCharacterMovement)) (== (Class|PaperFlipbookComponent|GetPlaybackPositioninFrames _sprite) 6))
            (bind _canuncrouch (CallFunction|CheckCeiling))
            (if (not _canuncrouch)
              (Class|PaperFlipbookComponent|SetPlaybackPositioninFrames _sprite 1 false)))))
      (:then_1
        (bind _canuncrouch_2 (CallFunction|CheckCeiling))
        (if _canuncrouch_2
          _
          (else
            (CallFunction|EndJump)))
        (if (not (Variables|Default|GetIsUsingAbility))
          (if (AI|Components|NavMovement|IsMovingonGround (Variables|Character|GetCharacterMovement))
            ;[1 1 1] Check for wall and set grounded animation state
            (bind _istouchingwall_2 (CallFunction|CheckforWall))
            (if _istouchingwall_2
              (Variables|Default|SetAnimState "NewEnumerator19")
              (else
                (Variables|Default|SetAnimState "NewEnumerator0")))
            (else
              ;[1 1 1] Check for wall and set arial animation state
              (bind _istouchingwall_3 (CallFunction|CheckforWall))
              (if _istouchingwall_3
                (Variables|Default|SetAnimState "NewEnumerator18")
                (else
                  (Variables|Default|SetAnimState "NewEnumerator1")))))
          (else
            ;[1 1 1] Set active ability based on AnimState so we know which hitbox to use
            (switch Utilities|FlowControl|Switch|SwitchonAnimStates (Variables|Default|GetAnimState)
              (:NewEnumerator3
                (Variables|Default|SetAbilityID 0))
              (:NewEnumerator4
                (Variables|Default|SetAbilityID 1)
                (CallFunction|StartAttack :!label _label))
              (:NewEnumerator8
                (Variables|Default|SetAbilityID 2))
              (:NewEnumerator10
                (Variables|Default|SetAbilityID 3)
                (goto _label))
              (:NewEnumerator20
                (Variables|Default|SetAbilityID 4))
              (:NewEnumerator21
                (Variables|Default|SetAbilityID 5))
              (:NewEnumerator22
                (Variables|Default|SetAbilityID 6))
              (:NewEnumerator23
                (Variables|Default|SetAbilityID 7))))))
      (:then_2
        (Utilities|FlowControl|Gate true
          (:Exit
            ;[1 1 1] Get attack's hitbox data based on AttackID
            (bind _imageindex (CallFunction|GetImageIndex))
            (if (and (<= _imageindex (Utilities|Array|Get(acopy) (Variables|Default|GetHitboxEndFrame) (Variables|Default|GetAbilityID))) (>= _imageindex (Utilities|Array|Get(acopy) (Variables|Default|GetHitboxStartFrame) (Variables|Default|GetAbilityID)))) ; Are we in an active frame?
              (CallFunction|PerformAbility)
              (else
                (CallFunction|EndAttack)))))))))

(event EventBeginPlay
  (bind _returnvalue (UserInterface|CreateWidget "/Game/Blueprints/System/UI/HUD.HUD_C" 0 0))
  (bind _output_get (Variables|Default|SetHUDReference _returnvalue))
  (UserInterface|Viewport|AddtoViewport _output_get 0)
  (Input|SetInputModeGameOnly (Game|GetPlayerController 0)))

(event EventBounce)

(event EventOnLanded
  (params (Hit :type Hit%20Result%20Structure%20%28by%20ref%29))
  ;[1 1 1] End arial attack when landing
  (if (Utilities|Enum|Equal(Enum) (Variables|Default|GetAnimState) "NewEnumerator4")
    (Variables|Default|SetAnimState "NewEnumerator0")
    (Variables|Default|SetIsUsingAbility false)))

(event EventRightAction
  ;[1 1 1] Response to attack input
  (if (or (Utilities|Enum|Equal(Enum) (Variables|Default|GetAnimState) "NewEnumerator0") (Utilities|Enum|Equal(Enum) (Variables|Default|GetAnimState) "NewEnumerator1")) ; Can only use attack in certain animation states
    (Variables|Default|SetAnimState "NewEnumerator4")
    (Variables|Default|SetIsUsingAbility true)))

(event EventDownAction
  ;[1 1 1] Response to attack input
  (if (or (Utilities|Enum|Equal(Enum) (Variables|Default|GetAnimState) "NewEnumerator0") (Utilities|Enum|Equal(Enum) (Variables|Default|GetAnimState) "NewEnumerator19"))
    (Variables|Default|SetAnimState "NewEnumerator10")
    (Variables|Default|SetIsUsingAbility true)
    (Character|Crouch)
    (Transformation|AddLocalOffset (Variables|Default|GetSprite) (Variables|Default|GetCrouchDisplacement) false false)
    (else
      (CallFunction|PassThroughPlatform))))

(event EventLeftAction
  ;[1 1 1] Response to attack input
  (Development|PrintString "LeftSwipe"))

(event EventUpAction
  ;[1 1 1] Response to attack input
  (Development|PrintString "UpSwipe"))

(event EventDeath
  (Variables|Default|SetIsDead true)
  (bind _asswift_game_mode (Utilities|Casting|CastToSwiftGameMode (Game|GetGameMode)))
  (Default|EndGame _asswift_game_mode)
  (Input|SetInputModeUIOnly (Game|GetPlayerController 0) (Variables|/Game/Blueprints/System/UI/GameEndMenu.GameEndMenu_C|GetRetryButton (Variables|/Game/Blueprints/System/SwiftGameMode.SwiftGameMode_C|GetGameEndMenuReference _asswift_game_mode)) "DoNotLock")
  (Actor|DestroyActor))

(event EventStartJump
  ;[1 1 1] Jumping Logic
  (if (and (not (Variables|Default|GetIsUsingAbility)) (Character|CanJump))
    (Character|Jump)))

(event EventEndJump
  ;[1 1 1] Jumping Logic
  (Character|StopJumping))

(fn ConstructionScript
  (Variables|Default|SetJumpMaxHoldTime (Variables|Default|GetMaxJumpHoldTime))
  (bind _output_get (Variables|Default|SetMaximumHealth 3))
  (Variables|Default|SetCurrentHealth _output_get))

(fn GetImageIndex
  (return (Class|PaperFlipbookComponent|GetPlaybackPositioninFrames (Variables|Default|GetSprite))))

(fn CheckforWall
  (bind _returnvalue (Transformation|GetActorLocation))
  ;[1 1 1] Linetrace from center of character to just outside of collision capsule. If hit actor is not a child of BaseCharacter then the player is touching a wall
  (bind (_outhit _returnvalue_2) (Collision|LineTraceByChannel _returnvalue (+ _returnvalue (Math|Vector|MakeVector (+ (Components|Capsule|GetScaledCapsuleRadius (Variables|Default|GetCapsuleComponent)) 1.0) 0.0 0.0)) "TraceTypeQuery1" false 0 "None"))
  (if _returnvalue_2
    (if (Utilities|ClassIsChildOf (Utilities|GetClass (.HitActor (Collision|BreakHitResult _outhit))) "/Game/Blueprints/Characters/BaseCharacter.BaseCharacter_C")
      (return false)
      (else
        (return true)))
    (else
      (return false))))

(fn PerformAbility
  (switch int (Variables|Default|GetAbilityID)
    (:1
      (CallFunction|SlashHitCheck))
    (:3
      (if (AI|Components|NavMovement|IsMovingonGround (Variables|Character|GetCharacterMovement))
        (CallFunction|SlideHitCheck)
        (else
          (Variables|Default|SetIsUsingAbility false)
          (Character|UnCrouch)
          (Transformation|AddLocalOffset (Variables|Default|GetSprite) (* (Variables|Default|GetCrouchDisplacement) -1.0) false false)
          (Variables|Default|SetAnimState "NewEnumerator1"))))))

(fn SlashHitCheck
  (bind _returnvalue (Transformation|GetActorLocation))
  (bind (_x _y _z) (Math|Vector|BreakVector _returnvalue))
  (bind (_x_2 _y_2 _z_2) (Math|Vector|BreakVector _returnvalue))
  (bind (_outhit _returnvalue_2) (Class|KismetSystemLibrary|BoxTraceSingleforObjects (Math|Vector|MakeVector _x_2 _y_2 (- _z_2 5.0)) (Math|Vector|MakeVector (+ _x 1e+02) _y (- _z 5.0)) "0.000000,100.000000,10.000000" "0, 0, 0" (Utilities|Array|MakeArray "ObjectTypeQuery3") false (Utilities|Array|MakeArray self) "None" true))
  (if _returnvalue_2
    (if (Utilities|ClassIsChildOf (Utilities|GetClass (.HitActor (Collision|BreakHitResult _outhit))) "/Game/Blueprints/Characters/BaseCharacter.BaseCharacter_C")
      (bind _asbase_character (Utilities|Casting|CastToBaseCharacter (.HitActor (Collision|BreakHitResult _outhit))))
      (Default|TakeDamage _asbase_character))))

(fn SlideHitCheck
  (bind _returnvalue (Transformation|GetActorLocation))
  (bind (_x _y _z) (Math|Vector|BreakVector _returnvalue))
  (bind (_x_2 _y_2 _z_2) (Math|Vector|BreakVector _returnvalue))
  (bind (_outhit _returnvalue_2) (Class|KismetSystemLibrary|BoxTraceSingleforObjects (Math|Vector|MakeVector _x_2 _y_2 (- _z_2 12.0)) (Math|Vector|MakeVector (+ _x 8e+01) _y (- _z 12.0)) "0.000000,50.000000,20.000000" "0, 0, 0" (Utilities|Array|MakeArray "ObjectTypeQuery3") false (Utilities|Array|MakeArray self) "None" true))
  (if _returnvalue_2
    (if (Utilities|ClassIsChildOf (Utilities|GetClass (.HitActor (Collision|BreakHitResult _outhit))) "/Game/Blueprints/Characters/BaseCharacter.BaseCharacter_C")
      (bind _asbase_character (Utilities|Casting|CastToBaseCharacter (.HitActor (Collision|BreakHitResult _outhit))))
      (Default|TakeDamage _asbase_character)
      (CallFunction|Bounce))))

(fn CheckCeiling
  (bind _returnvalue (Transformation|GetActorLocation))
  (bind _returnvalue_2 (Collision|LineTraceByChannel _returnvalue (+ _returnvalue (Math|Vector|MakeVector 0.0 0.0 (+ (Components|Capsule|GetScaledCapsuleRadius (Variables|Default|GetCapsuleComponent)) 21.0))) "TraceTypeQuery1" false 0 "None"))
  (if _returnvalue_2
    (return false)
    (else
      (return true))))